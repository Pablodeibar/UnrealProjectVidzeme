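; BPC_Inventory is an inventory component that stores picked items for its owning BP_ThirdPersonCharacter.
; Adding an item appends it to the Inventory array and pushes it to the character's inventory widget.
; Using an item searches for the hard-coded "Chicken" entry, calls the character's UseItem and removes that entry.
; An ItemUsed flag blocks further use after the first success and is never reset here.
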(fn AddItemtoInventory
  (params (NewItem :type String%20%28by%20ref%29))
  (Utilities|Array|Add (Variables|Default|GetInventory) NewItem)
  (bind _asbp_third_person_character (Utilities|Casting|CastToBP_ThirdPersonCharacter (Components|GetOwner)))
  (Default|AddItemtoUI (Variables|/Game/ThirdPerson/Blueprints/BP_ThirdPersonCharacter.BP_ThirdPersonCharacter_C|GetInventoryWidget _asbp_third_person_character) NewItem))

(fn UseItemfromInventory
  (bind _inventory (Variables|Default|GetInventory))
  (if (not (Variables|Default|GetItemUsed))
    (bind (_array_element _array_index) (Utilities|Array|ForEachLoopwithBreak _inventory :!label _label)
      (:LoopBody
        (if (Utilities|Enum|Equal(Enum) _array_element "Chicken")
          (bind _asbp_third_person_character (Utilities|Casting|CastToBP_ThirdPersonCharacter (Components|GetOwner)))
          (Default|UseItem _asbp_third_person_character)
          (Utilities|Array|RemoveIndex _inventory _array_index)
          (Variables|Default|SetItemUsed true)
          (goto _label Break))))))