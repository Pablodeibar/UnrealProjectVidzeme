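; GMBP_WinCondition tracks special NPC deaths and shows the win screen once two have been killed.
; Its NPC_Death event increments the kill counter, prints it, and adds WBP_WinScreen to the viewport when the count equals two.
; A node to disable player input is left unconnected, so this Blueprint does not disable input on a win.
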(event Custom|NPC_Death
  (Variables|Default|SetSpecialNPCKilled (+ (Variables|Default|GetSpecialNPCKilled) 1))
  (Development|PrintString (Utilities|String|ToString(Integer) (Variables|Default|GetSpecialNPCKilled)))
  (if (== 2 (Variables|Default|GetSpecialNPCKilled))
    (bind _returnvalue (UserInterface|CreateWidget "/Game/BluePrints/WBP_WinScreen.WBP_WinScreen_C"))
    (UserInterface|Viewport|AddtoViewport _returnvalue 0)))

(event EventBeginPlay)

(event EventTick
  (params (DeltaSeconds :type Float%20%28single-precision%29)))

(fn ConstructionScript)