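; Special target NPC that counts toward the win condition when killed, with a randomized look.
; The construction script picks a random skeletal mesh and skin, pant and jacket materials.
; BeginPlay starts a scripted walk: after a random delay, it moves through two hardcoded points via AI MoveTo, tracked by IsMoving.
; Lethal damage plays a sound, notifies GMBP_WinCondition, ragdolls the mesh, then destroys the actor after a delay.
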(event Custom|NPC_Path
  (bind _self self)
  (Utilities|FlowControl|Delay (Math|Random|RandomFloatinRange 1.0 3.0))
  (Variables|Default|SetIsMoving? true)
  (AI|AIMoveTo _self "-18296.000000,-3616.000000,188.000000" 0 5.0 false
    (:OnSuccess
      (AI|AIMoveTo _self "-15809.000000,-3837.000000,188.000000" 0 5.0 false
        (:OnSuccess
          _)
        (:OnFail
          _))
      (Variables|Default|SetIsMoving? false))))

(event Collision|EventActorBeginOverlap
  (params (OtherActor :type Actor%20Object%20Reference)))

(event Game|Damage|EventAnyDamage
  (params (Damage :type Float%20%28single-precision%29) (DamageType :type Damage%20Type%20Object%20Reference) (InstigatedBy :type Controller%20Object%20Reference) (DamageCauser :type Actor%20Object%20Reference))
  (bind _mesh (Variables|Character|GetMesh))
  ;[1 1 1] Health - handle health of character
  (if (> (Variables|Default|GetHealth) 0.0)
    (Variables|Default|SetHealth (- (Variables|Default|GetHealth) Damage))
    (if (<= (Variables|Default|GetHealth) 0.0)
      ;[1 1 1] Play a sound when he die
      (Audio|PlaySoundatLocation "/Game/Assets/Sounds/NPCDeath.NPCDeath" (Transformation|GetActorLocation) "0, 0, 0" 1.0 1.0 0.0 0 0 0 0)
      ;[1 1 1] Inclement the number of special NPC killed
      (bind _asgmbp_win_condition (Utilities|Casting|CastToGMBP_WinCondition (Game|GetGameMode)))
      (Default|NPCDeath _asgmbp_win_condition)
      (Physics|SetSimulatePhysics _mesh true)
      (Class|SkeletalMeshComponent|SetPhysicsBlendWeight _mesh 1.0)
      (Collision|SetCollisionEnabled _mesh "QueryAndPhysics")
      (Utilities|FlowControl|Delay 5.0)
      (Actor|DestroyActor))))

(event EventTick
  (params (DeltaSeconds :type Float%20%28single-precision%29)))

(event EventBeginPlay
  (Utilities|FlowControl|Sequence
    (:then_0
      (CallFunction|NPCPath))))

(fn ConstructionScript
  (bind _jacketref (Variables|Default|GetJacketRef))
  (bind _skeletonref (Variables|Default|GetSkeletonRef))
  (bind _skinref (Variables|Default|GetSkinRef))
  (bind _pantref (Variables|Default|GetPantRef))
  (Components|SkeletalMesh|SetSkeletalMeshAsset (Variables|Character|GetMesh) (Utilities|Array|Get(acopy) _skeletonref (Math|Random|RandomInteger (Utilities|Array|Length _skeletonref))))
  (Rendering|Material|CreateDynamicMaterialInstance (Variables|Character|GetMesh) 2 (Utilities|Array|Get(acopy) _skinref (Math|Random|RandomInteger (Utilities|Array|Length _skinref))) "None" :!class /Script/Engine.PrimitiveComponent)
  (Rendering|Material|CreateDynamicMaterialInstance (Variables|Character|GetMesh) 0 (Utilities|Array|Get(acopy) _pantref (Math|Random|RandomInteger (Utilities|Array|Length _pantref))) "None" :!class /Script/Engine.PrimitiveComponent)
  (Rendering|Material|CreateDynamicMaterialInstance (Variables|Character|GetMesh) 1 (Utilities|Array|Get(acopy) _jacketref (Math|Random|RandomInteger (Utilities|Array|Length _jacketref))) "None" :!class /Script/Engine.PrimitiveComponent))