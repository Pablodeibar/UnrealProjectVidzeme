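; Special killable NPC whose death counts toward the win condition.
; On BeginPlay it loops one of three animations chosen by WhoIAm.
; Damage drains Health; at zero it plays a death sound, notifies GMBP_WinCondition, ragdolls the mesh and destroys itself after a delay.
; Random skeleton and clothing material logic exists but is disconnected from the empty construction script.
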(event Game|Damage|EventAnyDamage
  (params (Damage :type Float%20%28single-precision%29) (DamageType :type Damage%20Type%20Object%20Reference) (InstigatedBy :type Controller%20Object%20Reference) (DamageCauser :type Actor%20Object%20Reference))
  (bind _mesh (Variables|Character|GetMesh))
  ;[1 1 1] Health - handle health of character
  (if (> (Variables|Default|GetHealth) 0.0)
    (Variables|Default|SetHealth (- (Variables|Default|GetHealth) Damage))
    (if (<= (Variables|Default|GetHealth) 0.0)
      ;[1 1 1] Play a sound when he die
      (Audio|PlaySoundatLocation "/Game/Assets/Sounds/NPCDeath.NPCDeath" (Transformation|GetActorLocation) "0, 0, 0" 1.0 1.0 0.0 0 0 0 0)
      ;[1 1 1] Inclement the number of special NPC killed
      (bind _asgmbp_win_condition (Utilities|Casting|CastToGMBP_WinCondition (Game|GetGameMode)))
      (Default|NPCDeath _asgmbp_win_condition)
      (Physics|SetSimulatePhysics _mesh true)
      (Class|SkeletalMeshComponent|SetPhysicsBlendWeight _mesh 1.0)
      (Collision|SetCollisionEnabled _mesh "QueryAndPhysics")
      (Utilities|FlowControl|Delay 5.0)
      (Actor|DestroyActor))))

(event EventBeginPlay
  (switch int (Variables|Default|GetWhoIAm?)
    (:0
      (Components|Animation|PlayAnimation (Variables|Character|GetMesh) "/Game/AnimStarterPack/Aim_Space_Hip.Aim_Space_Hip" true))
    (:1
      (Components|Animation|PlayAnimation (Variables|Character|GetMesh) "/Game/NPC/Animations/A_TalkingMan.A_TalkingMan" true))
    (:2
      (Components|Animation|PlayAnimation (Variables|Character|GetMesh) "/Game/NPC/Animations/A_ShowingBoxe.A_ShowingBoxe" true))))

(fn ConstructionScript)