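; BP_NPCDialog is an NPC actor that offers voiced, row-by-row dialog to the third-person character.
; Entering its Box reveals a TextRender and creates a WBP_DialogUI widget; leaving hides and removes them.
; Eventdialogoccurs, not called in this graph, passes NPCText to the widget, plays the next row's sound and advances TextRow, removing the widget after the last row.
; A DoOnce guards each step and is immediately reset through ResetDialog.
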(event OnComponentBeginOverlap(Box)
  (params (OverlappedComponent :type Primitive%20Component%20Object%20Reference) (OtherActor :type Actor%20Object%20Reference) (OtherComp :type Primitive%20Component%20Object%20Reference) (OtherBodyIndex :type Integer) (bFromSweep :type Boolean) (SweepResult :type Hit%20Result%20Structure%20%28by%20ref%29))
  ;[1 1 1] Handle appear dialog
  (Utilities|Casting|CastToBP_ThirdPersonCharacter OtherActor)
  (Development|SetHiddeninGame (Variables|Default|GetTextRender) false false)
  (bind _returnvalue (UserInterface|CreateWidget "/Game/BluePrints/WBP_DialogUI.WBP_DialogUI_C"))
  (bind _output_get (Variables|Default|SetDialogUI _returnvalue))
  (UserInterface|Viewport|AddtoViewport _output_get 0))

(event OnComponentEndOverlap(Box)
  (params (OverlappedComponent :type Primitive%20Component%20Object%20Reference) (OtherActor :type Actor%20Object%20Reference) (OtherComp :type Primitive%20Component%20Object%20Reference) (OtherBodyIndex :type Integer))
  (bind _dialogui (Variables|Default|GetDialogUI))
  ;[1 1 1] Handle disappear dialog
  (Utilities|Casting|CastToBP_ThirdPersonCharacter OtherActor)
  (Development|SetHiddeninGame (Variables|Default|GetTextRender) true false)
  (Utilities|IsValid _dialogui
    (:Is%20Valid
      (Widget|RemovefromParent _dialogui))))

(event Custom|ResetDialog
  ;[1 1 1] Handle dialog content
  (Utilities|FlowControl|DoOnce false) ; enters at Reset
)

(event EventBeginPlay)

(event Collision|EventActorBeginOverlap
  (params (OtherActor :type Actor%20Object%20Reference)))

(event EventTick
  (params (DeltaSeconds :type Float%20%28single-precision%29)))

(event EventEventdialogoccurs
  ;[1 1 1] Handle dialog content
  (Utilities|FlowControl|DoOnce false
    (:Completed
      (Variables|/Game/BluePrints/WBP_DialogUI.WBP_DialogUI_C|Settext (Variables|Default|GetDialogUI) (Variables|Default|GetNPCText))
      (Audio|PlaySound2D (Utilities|Array|Get(acopy) (Variables|Default|GetNPCSounds) (+ (Variables|/Game/BluePrints/WBP_DialogUI.WBP_DialogUI_C|GettextRow (Variables|Default|GetDialogUI)) 1)) 1.0 1.0 0.0 0 0)
      (Widget|SetVisibility (Variables|/Game/BluePrints/WBP_DialogUI.WBP_DialogUI_C|GetTextBlock_0 (Variables|Default|GetDialogUI)) "Visible")
      (if (> (+ (Variables|/Game/BluePrints/WBP_DialogUI.WBP_DialogUI_C|GettextRow (Variables|Default|GetDialogUI)) 1) (- (Utilities|Array|Length (Variables|Default|GetNPCText)) 1))
        (Widget|RemovefromParent (Variables|Default|GetDialogUI))
        (CallFunction|ResetDialog)
        (else
          (Variables|/Game/BluePrints/WBP_DialogUI.WBP_DialogUI_C|SettextRow (Variables|Default|GetDialogUI) (+ (Variables|/Game/BluePrints/WBP_DialogUI.WBP_DialogUI_C|GettextRow (Variables|Default|GetDialogUI)) 1))
          (CallFunction|ResetDialog))))))

(fn ConstructionScript)