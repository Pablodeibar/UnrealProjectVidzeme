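; BP_AIChar is an AI character that carries a gun and shoots a given enemy.
; On BeginPlay it snaps the gun mesh to the body's weapon socket.
; ShootEnemy spawns an explosion particle at the gun socket, then line traces on the Camera channel from its own location to the enemy.
; Damage is applied, credited to its controller, only if the trace hits that enemy first.
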(event Custom|ShootEnemy
  (params (EnemyToShoot :type Actor%20Object%20Reference))
  ;[1 1 1] Handle shoot
  (CallFunction|PlayShootFx)
  (bind _outhit (Collision|LineTraceByChannel (Transformation|GetActorLocation) (Transformation|GetActorLocation EnemyToShoot) "TraceTypeQuery2" false 0 "None"))
  (if true
    (if (== (.HitActor (Collision|BreakHitResult _outhit)) EnemyToShoot)
      (Game|Damage|ApplyDamage (.HitActor (Collision|BreakHitResult _outhit)) 2e+01 (Pawn|GetController) self "/Script/Engine.DamageType"))))

(event Custom|PlayShootFx
  (bind _gunmesh (Variables|Default|GetGunMesh))
  ;[1 1 1] Spawn particles when shooting
  (Effects|SpawnEmitteratLocation "/Game/StarterContent/Particles/P_Explosion.P_Explosion" (Transformation|GetSocketLocation _gunmesh "Socket") (Transformation|GetSocketRotation _gunmesh "Socket")))

(event EventBeginPlay
  ;[1 1 1] Snap the gun on the grabpoint
  (Transformation|AttachComponentToComponent (Variables|Default|GetGunMesh) (Variables|Character|GetMesh) "WeaponSocket" "SnapToTarget" "SnapToTarget" "SnapToTarget" true))

(event Collision|EventActorBeginOverlap
  (params (OtherActor :type Actor%20Object%20Reference)))

(event EventTick
  (params (DeltaSeconds :type Float%20%28single-precision%29)))

(fn ConstructionScript)